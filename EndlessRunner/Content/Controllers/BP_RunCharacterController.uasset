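; BP_RunCharacterController is a controller that turns movement axis input into motion for the BP_RunCharacter pawn.
; On BeginPlay it casts the controlled pawn to BP_RunCharacter and caches the reference.
; The MoveForward and MoveRight axis events feed movement input along that character's forward and right vectors, scaled by the axis value.
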(event EventBeginPlay
  (bind _asbp_run_character (Utilities|Casting|CastToBP_RunCharacter (Pawn|GetControlledPawn)))
  (Variables|Default|SetBP%20Run%20Character _asbp_run_character))

(event EventTick
  (params (DeltaSeconds :type Float%20%28single-precision%29)))

(event Input|AxisEvents|InputAxisMoveForward
  (params (AxisValue :type Float%20%28single-precision%29))
  (bind _bp_run_character (Variables|Default|GetBP%20Run%20Character))
  (Pawn|Input|AddMovementInput _bp_run_character (Transformation|GetActorForwardVector _bp_run_character) AxisValue false))

(event Input|AxisEvents|InputAxisMoveRight
  (params (AxisValue :type Float%20%28single-precision%29))
  (bind _bp_run_character (Variables|Default|GetBP%20Run%20Character))
  (Pawn|Input|AddMovementInput _bp_run_character (Transformation|GetActorRightVector _bp_run_character) AxisValue false))

(fn ConstructionScript)