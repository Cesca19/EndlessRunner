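; BP_RunGameMode is a game mode that builds an endless track from BP_FloorTile actors.
; On BeginPlay it spawns an initial run of tiles, each placed at the previous tile's attach transform.
; It binds to each tile's Exited event, and OnTileExited spawns the next tile, then destroys the exited one after a short delay.
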(event Custom|OnTileExited
  (params (Tile :type BP%20Floor%20Tile%20Object%20Reference))
  (CallFunction|SpawnNextTile)
  (Utilities|FlowControl|Delay 0.5)
  (Actor|DestroyActor Tile))

(event EventBeginPlay
  (CallFunction|SpawnTiles 4))

(event EventTick
  (params (DeltaSeconds :type Float%20%28single-precision%29)))

(fn ConstructionScript)

(fn SpawnNextTile
  (bind _returnvalue (Game|SpawnActorfromClass "/Game/Actors/BP_FloorTile.BP_FloorTile_C" (Variables|Default|GetCurrentStartTransform) "Undefined" "MultiplyWithRoot" 0 0))
  (EventDispatchers|BindEventtoExited _returnvalue (EventDispatchers|CreateEvent :!event Custom|OnTileExited))
  (bind _returnvalue_2 (Default|GetAttachTransform _returnvalue))
  (Variables|Default|SetCurrentStartTransform _returnvalue_2))

(fn SpawnTiles
  (params (Number :type Integer))
  (bind _result (Math|Integer|DecrementInt Number)
    (:%20%20
      (for _index (range 0 _result)
        (CallFunction|SpawnNextTile)))))