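; BP_RunCharacter is the player character for what appears to be a runner game, tracking collected coins and handling death.
; Overlapping a BP_CoinPickUp adds that pickup's value to the Coins total.
; Die disables input and movement, spawns an explosion effect and sound, sets IsDead, then calls PlayerDeath.
; GetIsDead exposes the death state, while a node to hide the mesh is left unconnected.
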(event Custom|Die
  (bind _returnvalue (Transformation|GetActorLocation))
  (Input|DisableInput 0)
  (Pawn|Components|CharacterMovement|DisableMovement (Variables|Character|GetCharacterMovement))
  (Effects|SpawnEmitteratLocation "/Game/StarterContent/Particles/P_Explosion.P_Explosion" _returnvalue "0, 0, 0" "2.000000,2.000000,2.000000")
  (Audio|SpawnSoundatLocation "/Game/StarterContent/Audio/Explosion02.Explosion02" _returnvalue "0, 0, 0" 1.0 1.0 0.0 0 0)
  (Variables|Default|SetIsDead true)
  (Default|CallPlayerDeath))

(event EventBeginPlay)

(event EventTick
  (params (DeltaSeconds :type Float%20%28single-precision%29)))

(event Collision|EventActorBeginOverlap
  (params (OtherActor :type Actor%20Object%20Reference))
  (bind _asbp_coin_pick_up (Utilities|Casting|CastToBP_CoinPickUp OtherActor))
  (bind _value (Default|GetValue _asbp_coin_pick_up))
  (Variables|Default|SetCoins (+ (Variables|Default|GetCoins) _value)))

(fn ConstructionScript)

(fn GetIsDead
  (return (Variables|Default|GetIsDead)))