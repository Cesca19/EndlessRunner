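; BP_FloorTile is a floor segment that populates itself with a random obstacle and reports when a character reaches its trigger.
; On BeginPlay it spawns a random ObstacleTypes entry at a random point in an offset box sized by BoxFloor, then attaches it to the tile root.
; A Character overlapping Box fires the Exited dispatcher, and GetAttachTransform exposes the Arrow's world transform as an attach point.
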(event OnComponentBeginOverlap(Box)
  (params (OverlappedComponent :type Primitive%20Component%20Object%20Reference) (OtherActor :type Actor%20Object%20Reference) (OtherComp :type Primitive%20Component%20Object%20Reference) (OtherBodyIndex :type Integer) (bFromSweep :type Boolean) (SweepResult :type Hit%20Result%20Structure%20%28by%20ref%29))
  (Utilities|Casting|CastToCharacter OtherActor)
  (Default|CallExited self))

(event EventBeginPlay
  (CallFunction|SpawnObstacle))

(event Collision|EventActorBeginOverlap
  (params (OtherActor :type Actor%20Object%20Reference)))

(event EventTick
  (params (DeltaSeconds :type Float%20%28single-precision%29)))

(fn ConstructionScript)

(fn GetAttachTransform
  (return (Transformation|GetWorldTransform (Variables|Default|GetArrow))))

(fn SpawnTransform
  (return (Math|Random|RandomPointinBoundingBox (+ (Transformation|GetWorldLocation (Variables|Default|GetDefaultSceneRoot)) "-500.000000,-500.000000,0.000000") (Variables|/Script/Engine.BoxComponent|GetBoxExtent (Variables|Default|GetBoxFloor)))))

(fn SpawnObstacle
  (bind _returnvalue (CallFunction|SpawnTransform))
  (bind _returnvalue_2 (Game|SpawnActorfromClass (.OutItem (Utilities|Array|Random (Variables|Default|GetObstacleTypes))) (Math|Conversions|ToTransform(Vector) _returnvalue) "Undefined" "MultiplyWithRoot" 0 0))
  (Transformation|AttachComponentToComponent _returnvalue_2 (Variables|Default|GetDefaultSceneRoot self) "None" "KeepWorld" "KeepWorld" "KeepWorld" true))